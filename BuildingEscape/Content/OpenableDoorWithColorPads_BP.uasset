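; A door actor that swings open and closed in response to OnOpen and OnClose events from OpenDoorWithColorPads.
; A timeline plays forward or in reverse, adding its OpenAngle yaw to the rotation cached at BeginPlay.
; An event track on the timeline toggles IsOpen and spawns either the lock or the close sound at the door's location.
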(event OnOpen(OpenDoorWithColorPads)
  (bind _returnvalue (Transformation|GetActorLocation))
  (bind _open_angle (Timeline|Timeline_0 Play)
    (:Update
      (Transformation|SetActorRotation (Math|Rotator|CombineRotators (Math|Rotator|MakeRotator 0.0 0.0 _open_angle) (Variables|Default|GetInitial%20Rotation))))
    (:PlayOpenSound
      (if (Variables|Default|GetIsOpen)
        (Audio|SpawnSoundatLocation "/Game/Audio/door_close.door_close" _returnvalue)
        (Variables|Default|SetIsOpen false)
        (else
          (Audio|SpawnSoundatLocation "/Game/Audio/door-lock.door-lock" _returnvalue)
          (Variables|Default|SetIsOpen true))))))

(event OnClose(OpenDoorWithColorPads)
  (bind _returnvalue (Transformation|GetActorLocation))
  (bind _open_angle (Timeline|Timeline_0 Reverse)
    (:Update
      (Transformation|SetActorRotation (Math|Rotator|CombineRotators (Math|Rotator|MakeRotator 0.0 0.0 _open_angle) (Variables|Default|GetInitial%20Rotation))))
    (:PlayOpenSound
      (if (Variables|Default|GetIsOpen)
        (Audio|SpawnSoundatLocation "/Game/Audio/door_close.door_close" _returnvalue)
        (Variables|Default|SetIsOpen false)
        (else
          (Audio|SpawnSoundatLocation "/Game/Audio/door-lock.door-lock" _returnvalue)
          (Variables|Default|SetIsOpen true))))))

(event EventBeginPlay
  (Variables|Default|SetInitial%20Rotation (Transformation|GetActorRotation)))

(fn ConstructionScript)